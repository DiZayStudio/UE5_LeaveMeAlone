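; BP_Save is the save game object that records the last score and the high score in separate slots, Score and ScoreMax.
; SaveScore always writes the Score slot, and overwrites ScoreMax only when the new score beats the stored one.
; Without an existing ScoreMax save, it writes both slots, using a newly created object for Score and itself for ScoreMax.
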(fn SaveScore
  (params (Score :type Integer))
  (bind _self self)
  (bind _returnvalue (SaveGame|DoesSaveGameExist "ScoreMax"))
  (if _returnvalue
    (bind _returnvalue_2 (SaveGame|LoadGamefromSlot "ScoreMax"))
    (bind _asbp_save (Utilities|Casting|CastToBP_Save _returnvalue_2))
    (if (< (Variables|BP_Save_C|GetScoreMax _asbp_save) Score)
      (Variables|Default|SetScore Score)
      (SaveGame|SaveGametoSlot _self "Score")
      (Variables|Default|SetScoreMax Score)
      (SaveGame|SaveGametoSlot _self "ScoreMax")
      (else
        (Variables|Default|SetScore Score)
        (SaveGame|SaveGametoSlot _self "Score")))
    (else
      (bind _returnvalue_3 (SaveGame|CreateSaveGameObject "BP_Save_C"))
      (Variables|BP_Save_C|SetScore _returnvalue_3 Score)
      (SaveGame|SaveGametoSlot _returnvalue_3 "Score")
      (Variables|Default|SetScoreMax Score)
      (SaveGame|SaveGametoSlot _returnvalue_3 "ScoreMax"))))